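; Runtime transform-gizmo actor that lets the player click objects and translate, rotate or scale them.
; It enables input and the mouse cursor on begin play, then maps hotkeys to transform mode, local/world space and component-based toggling.
; Left click traces static and dynamic world objects, with Shift appending to the selection, and release clears the active gizmo domain.
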(event `Key|Tab`
  (params (Key :type "Key Structure"))
  (:`Pressed`
    (switch `ESpaceType` (`self.CurrentSpaceType`)
      (:`ST_None`
        (`self.SetSpaceType` "ST_World" :!label _label))
      (:`ST_Local`
        (goto _label))
      (:`ST_World`
        (`self.SetSpaceType` "ST_Local")))))

(event `self.ReceiveBeginPlay`
  (bind _returnvalue (`GameplayStatics.GetPlayerController` 0))
  (`self.EnableInput` _returnvalue)
  (set `PlayerController.bShowMouseCursor` true _returnvalue))

(event `Key|Q`
  (params (Key :type "Key Structure"))
  (:`Pressed`
    (`self.SetTransformationType` "TT_Translation")))

(event `Key|LeftMouseButton`
  (params (Key :type "Key Structure"))
  (:`Pressed`
    (`self.MouseTraceByObjectTypes` 1000.0 (`|MakeArray` "ECC_WorldDynamic" "ECC_WorldStatic" :!type "ECollisionChannel Enum") (`|MakeArray` self :!type "Actor Object Reference") (`KismetInputLibrary.ModifierKeysState_IsShiftDown` (`KismetInputLibrary.GetModifierKeysState`)) true))
  (:`Released`
    (`self.ClearDomain`)))

(event `Key|E`
  (params (Key :type "Key Structure"))
  (:`Pressed`
    (`self.SetTransformationType` "TT_Rotation")))

(event `Key|R`
  (params (Key :type "Key Structure"))
  (:`Pressed`
    (`self.SetTransformationType` "TT_Scale")))

(event `Key|T`
  (params (Key :type "Key Structure"))
  (:`Pressed`
    (`self.SetComponentBased` (not (`self.bComponentBased`)))))

(fn `UserConstructionScript`)